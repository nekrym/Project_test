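; BP_Gate_ZloyAdolf is an interactive gate that swings on its yaw axis when the player uses an input action.
; Box overlap enables and disables player 0's input on the actor, without checking which actor overlaps.
; ActionOpenAndCloseGate flips ClosedGate to play or reverse the Gate timeline, which rotates Gate32.
; Timeline updates also overwrite ClosedGate from a near-end angle threshold.
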(event `self.Box.OnComponentBeginOverlap`
  (params (OverlappedComponent :type "PrimitiveComponent Object Reference") (OtherActor :type "Actor Object Reference") (OtherComp :type "PrimitiveComponent Object Reference") (OtherBodyIndex :type Integer) (bFromSweep :type Boolean) (SweepResult :type "HitResult Structure (by ref)"))
  (`self.EnableInput` (`GameplayStatics.GetPlayerController` 0)))

(event `self.Box.OnComponentEndOverlap`
  (params (OverlappedComponent :type "PrimitiveComponent Object Reference") (OtherActor :type "Actor Object Reference") (OtherComp :type "PrimitiveComponent Object Reference") (OtherBodyIndex :type Integer))
  (`self.DisableInput` (`GameplayStatics.GetPlayerController` 0)))

(event `InputAction|ActionOpenAndCloseGate`
  (params (Key :type "Key Structure"))
  (:`Pressed`
    (bind _output_get (set `self.ClosedGate` (not (`self.ClosedGate`))))
    (if _output_get
      (bind (_direction _newtrack_0) (`Timeline|Gate` :!label _label)
        (:`Update`
          (`SceneComponent.K2_SetRelativeRotation` (`self.Gate32`) (`KismetMathLibrary.MakeRotator` 0.0 0.0 _newtrack_0) false false)
          (set `self.ClosedGate` (> _newtrack_0 59.0))))
      (else
        (goto _label :!via `Reverse`)))))

(fn `UserConstructionScript`)