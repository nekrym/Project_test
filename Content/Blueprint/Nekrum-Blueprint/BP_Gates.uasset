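; BP_Gates is an interactive double gate that the player opens and closes with the ActionOpenAndCloseGate input.
; A Box trigger enables the actor's input for player 0 on any overlap and disables it on exit.
; Each press flips ClosedGate and instantly snaps both leaves to opposite 90-degree yaws or back to zero, without interpolation.
; Despite its name, ClosedGate is true in the swung-open state.
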(event `self.Box.OnComponentBeginOverlap`
  (params (OverlappedComponent :type "PrimitiveComponent Object Reference") (OtherActor :type "Actor Object Reference") (OtherComp :type "PrimitiveComponent Object Reference") (OtherBodyIndex :type Integer) (bFromSweep :type Boolean) (SweepResult :type "HitResult Structure (by ref)"))
  (`self.EnableInput` (`GameplayStatics.GetPlayerController` 0)))

(event `self.Box.OnComponentEndOverlap`
  (params (OverlappedComponent :type "PrimitiveComponent Object Reference") (OtherActor :type "Actor Object Reference") (OtherComp :type "PrimitiveComponent Object Reference") (OtherBodyIndex :type Integer))
  (`self.DisableInput` (`GameplayStatics.GetPlayerController` 0)))

(event `InputAction|ActionOpenAndCloseGate`
  (params (Key :type "Key Structure"))
  (:`Pressed`
    (bind _output_get (set `self.ClosedGate` (not (`self.ClosedGate`))))
    (if _output_get
      (`|ExecutionSequence`
        (:`then_0`
          (`SceneComponent.K2_SetRelativeRotation` (`self.BP_Gate331`) (`KismetMathLibrary.MakeRotator` 0.0 0.0 (+ 90.0 0.0)) false false)
          (set `self.ClosedGate` (> 89.0 0.0)))
        (:`then_1`
          (`SceneComponent.K2_SetRelativeRotation` (`self.Gate34`) (`KismetMathLibrary.MakeRotator` 0.0 0.0 (- 0.0 90.0)) false false)))
      (else
        (`|ExecutionSequence`
          (:`then_0`
            (`SceneComponent.K2_SetRelativeRotation` (`self.BP_Gate331`) (`KismetMathLibrary.MakeRotator` 0.0) false false))
          (:`then_1`
            (`SceneComponent.K2_SetRelativeRotation` (`self.Gate34`) (`KismetMathLibrary.MakeRotator` 0.0) false false)))))))

(fn `UserConstructionScript`)